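; Double door actor that swings its two leaves open in opposite directions when interacted with or when a Player-tagged actor enters its box trigger.
; A timeline lerps the leaves' yaw from zero to plus and minus 90 degrees, flipping IsClosed when finished.
; Interact plays or reverses the timeline based on IsClosed, while the trigger only plays it forward.
; IsInteractable always returns true and DestroyDoor is an empty stub.
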(event `self.ReceiveBeginPlay`)

(event `self.Interact`
  (params (Interactor :type "ASCharacter Object Reference"))
  (if true
    (if (`self.IsClosed`)
      (bind (_direction _alpha) (`Timeline|Timeline` :!label _label)
        (:`Update`
          (`SceneComponent.K2_SetRelativeRotation` (`self.SM_Doors`) (`KismetMathLibrary.MakeRotator` 0.0 0.0 (`KismetMathLibrary.Lerp` 0.0 (* 90.0 -1.0) _alpha)) false false)
          (`SceneComponent.K2_SetRelativeRotation` (`self.SM_Doors1`) (`KismetMathLibrary.MakeRotator` 0.0 0.0 (`KismetMathLibrary.Lerp` 0.0 90.0 _alpha)) false false))
        (:`Finished`
          (set `self.IsClosed` (not (`self.IsClosed`)))))
      (else
        (goto _label :!via `ReverseFromEnd`)))))

(event `self.Box.OnComponentBeginOverlap`
  (params (OverlappedComponent :type "PrimitiveComponent Object Reference") (OtherActor :type "Actor Object Reference") (OtherComp :type "PrimitiveComponent Object Reference") (OtherBodyIndex :type Integer) (bFromSweep :type Boolean) (SweepResult :type "HitResult Structure (by ref)"))
  (if (`self.ActorHasTag` OtherActor "Player")
    (goto _label)))

(fn `DestroyDoor`)

(fn `IsInteractable`
  (returns (ReturnValue :type Boolean))
  (return true))

(fn `UserConstructionScript`)