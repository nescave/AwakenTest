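; BP_GameStartNotifier is a trigger actor that starts a game round when the player leaves its area.
; A Box component's end-overlap event checks whether the departing actor carries the Player tag and, if so, calls StartRound on ASGame.
; BeginPlay, begin-overlap and Tick are disabled stubs, so the end-overlap handler is its only logic.
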(event `self.Box.OnComponentEndOverlap`
  (params (OverlappedComponent :type "PrimitiveComponent Object Reference") (OtherActor :type "Actor Object Reference") (OtherComp :type "PrimitiveComponent Object Reference") (OtherBodyIndex :type Integer))
  (if (`self.ActorHasTag` OtherActor "Player")
    (`ASGameMode.StartRound` (`self.ASGame`))))

(fn `UserConstructionScript`
  (`parent.UserConstructionScript`))