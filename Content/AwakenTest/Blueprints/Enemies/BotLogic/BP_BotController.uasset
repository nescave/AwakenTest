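; AI controller for enemy bots that runs BT_Enemy on possess and turns sight and hearing stimuli into blackboard state.
; Sight flags line of sight and alert, then enables shooting after a notice delay.
; Losing sight or hearing a target stores its last seen location and, if it is far enough away, starts a timer to stop shooting.
; Hearing events are ignored while sight is active.
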(event `self.ReceivePossess`
  (params (PossessedPawn :type "Pawn Object Reference"))
  (bind _asasbot_character (cast `ASBotCharacter` (`self.K2_GetPawn`)))
  (set `self.BotCharacter` _asasbot_character)
  (`self.RunBehaviorTree` "/Game/AwakenTest/Blueprints/Enemies/BotLogic/BT_Enemy.BT_Enemy"))

(event `self.OnSightStimulus`
  (params (Actor :type "Actor Object Reference") (Stimulus :type "AIStimulus Structure"))
  (bind _returnvalue (`AIBlueprintHelperLibrary.GetBlackboard` null))
  (`KismetSystemLibrary.K2_ClearAndInvalidateTimerHandle` (`self.DisableCanShootTimerHandle`))
  (`BlackboardComponent.SetValueAsBool` _returnvalue (`self.HasLineOfSight`) true)
  (`BlackboardComponent.SetValueAsBool` _returnvalue (`self.Alerted`) true)
  (bind _returnvalue_2 (`KismetSystemLibrary.K2_SetTimerDelegate` (delegate `StartShooting`) (`self.CanShootAfterNotice`)))
  (set `self.EnableCanShootTimerHandle` _returnvalue_2))

(event `StartShooting`
  (bind _returnvalue (`AIBlueprintHelperLibrary.GetBlackboard` null))
  (`BlackboardComponent.SetValueAsBool` _returnvalue (`self.CanShoot`) true)
  (`BlackboardComponent.SetValueAsBool` _returnvalue (`self.Alerted`) false))

(event `self.OnSightStimulusEnded`
  (params (Actor :type "Actor Object Reference") (Stimulus :type "AIStimulus Structure"))
  (bind _returnvalue (`self.GetTarget`))
  (bind _returnvalue_2 (`AIBlueprintHelperLibrary.GetBlackboard` null))
  (`KismetSystemLibrary.K2_ClearAndInvalidateTimerHandle` (`self.EnableCanShootTimerHandle`))
  (`BlackboardComponent.SetValueAsBool` _returnvalue_2 (`self.HasLineOfSight`) false)
  (`BlackboardComponent.SetValueAsBool` _returnvalue_2 (`self.Alerted`) true)
  (`/Engine/EditorBlueprintResources/StandardMacros.IsValid` _returnvalue
    (:`Is Valid`
      (`ASBotCharacter.SetLastSeenLocation` (`self.BotCharacter`) (`self.K2_GetActorLocation` _returnvalue))
      (if (> (`KismetMathLibrary.Vector_Distance` (`self.K2_GetActorLocation` (`self.GetTarget`)) (`self.K2_GetActorLocation` (`self.BotCharacter`))) 300.0) :!label _label
        (bind _returnvalue_3 (`KismetSystemLibrary.K2_SetTimerDelegate` (delegate `StopShooting`) 1.5))
        (set `self.DisableCanShootTimerHandle` _returnvalue_3)))))

(event `self.OnHearingStimulus`
  (params (Actor :type "Actor Object Reference") (Stimulus :type "AIStimulus Structure"))
  (if (not (`self.bActiveSightStimulus`))
    (`BlackboardComponent.SetValueAsBool` (`AIBlueprintHelperLibrary.GetBlackboard` null) (`self.Alerted`) true)
    (`ASBotCharacter.SetLastSeenLocation` (`self.BotCharacter`) (`self.K2_GetActorLocation` (`self.GetTarget`)))
    (goto _label)))

(event `StopShooting`
  (`BlackboardComponent.SetValueAsBool` (`AIBlueprintHelperLibrary.GetBlackboard` null) (`self.CanShoot`) false))

(event `self.OnHearingStimulusEnded`
  (params (Actor :type "Actor Object Reference") (Stimulus :type "AIStimulus Structure"))
  (if (not (`self.bActiveSightStimulus`))
    (`BlackboardComponent.SetValueAsBool` (`AIBlueprintHelperLibrary.GetBlackboard` null) (`self.Alerted`) false)
    (`/Engine/EditorBlueprintResources/StandardMacros.IsValid` (`self.GetTarget`)
      (:`Is Valid`
        (goto _label)))))

(fn `UserConstructionScript`)