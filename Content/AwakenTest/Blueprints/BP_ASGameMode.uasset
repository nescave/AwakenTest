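; BP_ASGameMode is a game mode that extends its parent's round events with end-of-round UI.
; Round end builds a W_EndRoundScreen through the cached BP_ASHUD's player controller, showing level cleared or failed with round times, and round reset removes it.
; BeginPlay also sets an announcement timer, cleared on round start, but its event is empty and the SendAnnouncement call is disconnected.
; Win, lose, kill and death events only call the parent.
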(event `self.ReceiveBeginPlay`
  (bind _asbp_ashud (cast `/Game/AwakenTest/Blueprints/BP_ASHUD` (`PlayerController.GetHUD` (`GameplayStatics.GetPlayerController` 0))))
  (set `self.ASHUD` _asbp_ashud)
  (bind _returnvalue (`KismetSystemLibrary.K2_SetTimerDelegate` (delegate `AddOnScreenAnnouncment`) 3.0))
  (set `self.AddAnnouncementHandle` _returnvalue))

(event `AddOnScreenAnnouncment`)

(event `self.OnRoundReset`
  (bind _scorewidget (`self.ScoreWidget`))
  (`parent.OnRoundReset`)
  (`/Engine/EditorBlueprintResources/StandardMacros.IsValid` _scorewidget
    (:`Is Valid`
      (`Widget.RemoveFromParent` _scorewidget))))

(event `self.OnRoundStart`
  (`parent.OnRoundStart`)
  (`KismetSystemLibrary.K2_ClearAndInvalidateTimerHandle` (`self.AddAnnouncementHandle`)))

(event `self.OnRoundEnd`
  (`parent.OnRoundEnd`)
  (bind _returnvalue (`self.CreateWinWidget`))
  (bind _output_get (set `self.ScoreWidget` _returnvalue))
  (`UserWidget.AddToViewport` _output_get 0))

(event `self.OnRoundWin`
  (`parent.OnRoundWin`))

(event `self.OnRoundLose`
  (`parent.OnRoundLose`))

(event `self.OnEnemyKilled`
  (`parent.OnEnemyKilled`))

(event `self.OnPlayerDeath`
  (`parent.OnPlayerDeath`))

(fn `CreateWinWidget`
  (returns (ReturnValue :type "/Game/AwakenTest/Blueprints/UI/W_EndRoundScreen Object Reference"))
  (bind _returnvalue (`self.GetRoundTime`))
  (bind _returnvalue_2 (`|CreateWidget` "/Game/AwakenTest/Blueprints/UI/W_EndRoundScreen.W_EndRoundScreen_C" (`HUD.GetOwningPlayerController` (`self.ASHUD`))))
  (if (`self.bRoundWon`)
    (`/Game/AwakenTest/Blueprints/UI/W_EndRoundScreen.SetWidgetData` _returnvalue_2 "Level Cleared" (`self.BestRoundTime`) _returnvalue)
    (else
      (`/Game/AwakenTest/Blueprints/UI/W_EndRoundScreen.SetWidgetData` _returnvalue_2 "Level Failed" 0.0 _returnvalue)))
  (return _returnvalue_2))

(fn `UserConstructionScript`)