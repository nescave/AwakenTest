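; BP_WorldMessage is a world-placed actor that shows a text message on screen while the player is inside its sphere.
; Sphere overlap by a Player-tagged pawn creates W_MessageFromAuthor with MessageText and hides the main widget of BP_ASHUD.
; End overlap, unfiltered by actor, removes the message and restores the main widget.
; Input mode and mouse cursor switching exists but is disconnected.
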(event `self.Sphere.OnComponentBeginOverlap`
  (params (OverlappedComponent :type "PrimitiveComponent Object Reference") (OtherActor :type "Actor Object Reference") (OtherComp :type "PrimitiveComponent Object Reference") (OtherBodyIndex :type Integer) (bFromSweep :type Boolean) (SweepResult :type "HitResult Structure (by ref)"))
  (if (`self.ActorHasTag` OtherActor "Player")
    (bind _aspawn (cast `Pawn` OtherActor))
    (bind _returnvalue (`Pawn.GetLocalViewingPlayerController` _aspawn))
    (set `self.PlayerController` _returnvalue)
    (bind _returnvalue_2 (`|CreateWidget` "/Game/AwakenTest/Blueprints/UI/W_MessageFromAuthor.W_MessageFromAuthor_C" _returnvalue))
    (bind _output_get (set `self.MessageWidget` _returnvalue_2))
    (`/Game/AwakenTest/Blueprints/UI/W_MessageFromAuthor.SetMessageText` _output_get (`self.MessageText`))
    (`UserWidget.AddToViewport` _output_get 0)
    (bind _asbp_ashud (cast `/Game/AwakenTest/Blueprints/BP_ASHUD` (`PlayerController.GetHUD` (`self.PlayerController`))))
    (bind _returnvalue_3 (`ASHUD.GetMainWidget` _asbp_ashud))
    (set `self.MainWidget` _returnvalue_3)
    (`Widget.SetVisibility` _returnvalue_3 "Hidden")))

(event `self.Sphere.OnComponentEndOverlap`
  (params (OverlappedComponent :type "PrimitiveComponent Object Reference") (OtherActor :type "Actor Object Reference") (OtherComp :type "PrimitiveComponent Object Reference") (OtherBodyIndex :type Integer))
  (bind _mainwidget (`self.MainWidget`))
  (`/Engine/EditorBlueprintResources/StandardMacros.IsValid` (`self.MessageWidget`)
    (:`Is Valid`
      (`Widget.RemoveFromParent` (`self.MessageWidget`))
      (`/Engine/EditorBlueprintResources/StandardMacros.IsValid` _mainwidget
        (:`Is Valid`
          (`Widget.SetVisibility` _mainwidget "Visible"))))))

(fn `UserConstructionScript`)