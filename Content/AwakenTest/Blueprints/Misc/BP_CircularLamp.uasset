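; BP_CircularLamp is a configurable lamp actor that pairs a circular band mesh with a spot light.
; Its construction script applies the shared color and intensity to both parts, and sets the light's attenuation radius.
; The band receives color in RGB and intensity in W as default custom primitive data, with no dynamic material instance created.
; The event graph holds no active logic.
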(fn `UserConstructionScript`
  (bind (_color_r _color_g _color_b) (break `LinearColor` (`self.Color`)))
  (bind _spotlight (`self.SpotLight`))
  (`PrimitiveComponent.SetDefaultCustomPrimitiveDataVector4` (`self.SM_CircularBand`) 0 (`KismetMathLibrary.MakeVector4` _color_r _color_g _color_b (`self.LightIntensity`)))
  (`LightComponent.SetLightColor` _spotlight (`self.Color`) true)
  (`LightComponent.SetIntensity` _spotlight (`self.LightIntensity`))
  (`LocalLightComponent.SetAttenuationRadius` _spotlight (`self.AttenRadius`)))